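; BP_AI is an AI character Blueprint that handles hit reactions for stun and knockdown.
; ApplyStun sets IsStunned and plays the punched montage, then a short timer calls ClearStun to reset the flag.
; ApplyKnockDown only clears focus on the AIC_AI controller.
; BeginPlay binds a health-change handler, which is currently empty.
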(event `self.ReceiveBeginPlay`
  (add `self.OnHealthChanged` (delegate `HealthChanged`)))

(event `HealthChanged` :!signature `self.OnHealthChanged`
  (params (NewHealth :type "Float (single-precision)") (HealthDelta :type "Float (single-precision)")))

(event `self.ApplyStun`
  (set `self.bIsStunned` true)
  (`self.PlayAnimMontage` "/Game/Animations/AM_Punched.AM_Punched")
  (`KismetSystemLibrary.K2_SetTimerDelegate` (delegate `ClearStun`) 1.0 false true))

(event `ClearStun`
  (set `self.bIsStunned` false))

(event `self.ApplyKnockDown`
  (bind _asaic_ai (cast `/Game/AI/AIC_AI` (`self.GetController`)))
  (`AIController.K2_ClearFocus` _asaic_ai))

(fn `UserConstructionScript`)